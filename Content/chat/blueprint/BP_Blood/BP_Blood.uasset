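; BP_Blood is a level actor that raises a pool of blood as one of the game's random anomalies.
; On BeginPlay it checks BP_MyGameInstance and runs only when an anomaly is active and the random anomaly ID is 21.
; A timeline's Height track then lerps the relative Z of LiquidMesh upward.
; Each update also disables the mesh's collision and prints a debug string.
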(event `self.ReceiveBeginPlay`
  (`self.RaiseBlood`))

(event `RaiseBlood`
  (bind _asbp_my_game_instance (cast `/Game/chat/blueprint/BP_MyGameInstance` (`GameplayStatics.GetGameInstance`)))
  (if (`/Game/chat/blueprint/BP_MyGameInstance.HasAnomaly` _asbp_my_game_instance)
    (if (== (`/Game/chat/blueprint/BP_MyGameInstance.randomAnomaly` _asbp_my_game_instance) 21)
      (bind (_direction _height) (`Timeline|Timeline`)
        (:`Update`
          (`KismetSystemLibrary.PrintString` "Updating Blood")
          (`SceneComponent.K2_SetRelativeLocation` (`self.LiquidMesh`) (`KismetMathLibrary.MakeVector` 0.0 0.0 (`KismetMathLibrary.Lerp` -10.0 5.0 _height)) false false)
          (`PrimitiveComponent.SetCollisionEnabled` (`self.LiquidMesh`) "NoCollision"))))))

(fn `UserConstructionScript`)