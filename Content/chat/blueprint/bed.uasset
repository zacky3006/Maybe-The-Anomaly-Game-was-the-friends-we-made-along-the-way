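; Interactable bed actor that ends a round in what appears to be an anomaly-detection loop and reloads the home level.
; On InteractBed, it sets transition and interact flags on BP_MyGameInstance, then raises the level counter if an anomaly was present or resets it to zero otherwise.
; It has the game instance generate the next anomaly, then fades the camera out before opening the level.
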(event `InteractBed`
  (bind _asbp_my_game_instance (cast `/Game/chat/blueprint/BP_MyGameInstance` (`GameplayStatics.GetGameInstance`)))
  (set `/Game/chat/blueprint/BP_MyGameInstance.Istransition` true _asbp_my_game_instance)
  (set `/Game/chat/blueprint/BP_MyGameInstance.IsInteract` true _asbp_my_game_instance)
  (if (`/Game/chat/blueprint/BP_MyGameInstance.HasAnomaly` _asbp_my_game_instance)
    (set `/Game/chat/blueprint/BP_MyGameInstance.CurrentLevel` (+ (`/Game/chat/blueprint/BP_MyGameInstance.CurrentLevel` _asbp_my_game_instance) 1) _asbp_my_game_instance)
    (else
      (set `/Game/chat/blueprint/BP_MyGameInstance.CurrentLevel` 0 _asbp_my_game_instance)))
  (`/Game/chat/blueprint/BP_MyGameInstance.GenerateAnomaly` _asbp_my_game_instance)
  (`PlayerCameraManager.StartCameraFade` :`self` (`GameplayStatics.GetPlayerCameraManager` 0) :`ToAlpha` 1.0 :`Duration` 1.5 :`bHoldWhenFinished` true)
  (`KismetSystemLibrary.Delay` 1.5)
  (`GameplayStatics.OpenLevel` "home")
  (`KismetSystemLibrary.PrintString` "Bed Used"))

(fn `UserConstructionScript`)