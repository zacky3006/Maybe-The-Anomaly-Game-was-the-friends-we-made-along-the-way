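; BP_Anomaly_Move2 is an anomaly actor that relocates itself when its anomaly is the one selected.
; On BeginPlay it makes its display mesh visible and collidable, then moves to a hardcoded location if the game instance's HasAnomaly is set and RandomAnomaly matches its index.
; UpdateAnomaly only prints the flag and ignores its SetActive input.
; The construction script's mesh assignment is disconnected and never runs.
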(event `UpdateAnomaly`
  (params (setActive :type Boolean))
  (bind _asbp_my_game_instance (cast `/Game/chat/blueprint/BP_MyGameInstance` (`GameplayStatics.GetGameInstance`)))
  (`KismetSystemLibrary.PrintString` (`KismetStringLibrary.Conv_BoolToString` (`/Game/chat/blueprint/BP_MyGameInstance.HasAnomaly` _asbp_my_game_instance)))
  (if (`/Game/chat/blueprint/BP_MyGameInstance.HasAnomaly` _asbp_my_game_instance)
    _))

(event `self.ReceiveBeginPlay`
  (bind _meshdisplay (`self.MeshDisplay`))
  (`KismetSystemLibrary.PrintString` "BP_Anomaly BeginPlay")
  (`PrimitiveComponent.SetCollisionEnabled` _meshdisplay "QueryAndPhysics")
  (`SceneComponent.SetVisibility` _meshdisplay true false)
  (`self.UpdateAnomaly` false)
  (bind _asbp_my_game_instance (cast `/Game/chat/blueprint/BP_MyGameInstance` (`GameplayStatics.GetGameInstance`)))
  (if (`/Game/chat/blueprint/BP_MyGameInstance.HasAnomaly` _asbp_my_game_instance)
    (if (== (`/Game/chat/blueprint/BP_MyGameInstance.randomAnomaly` _asbp_my_game_instance) 24)
      (`self.K2_SetActorLocation` self (-2760.0 410.0 140.0) false false))))

(fn `UserConstructionScript`)