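; Door actor for an anomaly-loop game: using it advances or resets the player's level progress.
; On BeginPlay it destroys itself for two specific active anomalies.
; InteractDoor resets CurrentLevel in the GameInstance if an anomaly exists, otherwise increments it, then generates an anomaly, fades and reloads "home".
; The level-10 "Ending" check follows only the reset, so that branch never fires.
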(event `self.ReceiveBeginPlay`
  (bind _asbp_my_game_instance (cast `/Game/chat/blueprint/BP_MyGameInstance` (`GameplayStatics.GetGameInstance`)))
  (if (`/Game/chat/blueprint/BP_MyGameInstance.HasAnomaly` _asbp_my_game_instance)
    (if (or (== (`/Game/chat/blueprint/BP_MyGameInstance.randomAnomaly` _asbp_my_game_instance) 23) (== (`/Game/chat/blueprint/BP_MyGameInstance.randomAnomaly` _asbp_my_game_instance) 21))
      (`self.K2_DestroyActor`))))

(event `InteractDoor`
  (bind _asbp_my_game_instance (cast `/Game/chat/blueprint/BP_MyGameInstance` (`GameplayStatics.GetGameInstance`)))
  (set `/Game/chat/blueprint/BP_MyGameInstance.Istransition` true _asbp_my_game_instance)
  (set `/Game/chat/blueprint/BP_MyGameInstance.IsInteract` true _asbp_my_game_instance)
  (if (`/Game/chat/blueprint/BP_MyGameInstance.HasAnomaly` _asbp_my_game_instance)
    (set `/Game/chat/blueprint/BP_MyGameInstance.CurrentLevel` 0 _asbp_my_game_instance)
    (if (== (`/Game/chat/blueprint/BP_MyGameInstance.CurrentLevel` _asbp_my_game_instance) 10)
      (`PlayerCameraManager.StartCameraFade` (`GameplayStatics.GetPlayerCameraManager` 0) 0.0 1.0 2.0 (struct :`R` 1.0 :`G` 1.0 :`B` 1.0 :`A` 1.0) false true)
      (`KismetSystemLibrary.Delay` 2.0)
      (`GameplayStatics.OpenLevel` "Ending")
      (else
        (`/Game/chat/blueprint/BP_MyGameInstance.GenerateAnomaly` _asbp_my_game_instance :!label _label)
        (`PlayerCameraManager.StartCameraFade` :`self` (`GameplayStatics.GetPlayerCameraManager` 0) :`ToAlpha` 1.0 :`Duration` 1.5 :`bHoldWhenFinished` true)
        (`KismetSystemLibrary.Delay` 1.5)
        (`GameplayStatics.OpenLevel` "home")
        (`KismetSystemLibrary.PrintString` "Door Used")))
    (else
      (set `/Game/chat/blueprint/BP_MyGameInstance.CurrentLevel` (+ (`/Game/chat/blueprint/BP_MyGameInstance.CurrentLevel` _asbp_my_game_instance) 1) _asbp_my_game_instance)
      (goto _label))))

(fn `UserConstructionScript`)