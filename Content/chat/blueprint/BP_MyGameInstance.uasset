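; Game instance Blueprint that decides whether the current level has an anomaly and which numbered anomaly it is.
; Init fills an array with anomaly numbers up to AnomalyNum.
; GenerateAnomaly always leaves level 0 clean, otherwise flips a random boolean and draws without replacement, calling ResetArray to refill the pool when empty.
; Debug prints report the removed number and the remaining pool.
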(event `self.ReceiveInit`
  (for _index (range 1 (+ (`self.anomalyNum`) 1))
    (`KismetArrayLibrary.Array_Add` (`self.Anomaly_array`) _index)))

(fn `GenerateAnomaly`
  (bind _anomaly_array (`self.Anomaly_array`))
  (bind _returnvalue (`KismetArrayLibrary.Array_Length` _anomaly_array))
  (if (== (`self.CurrentLevel`) 0)
    (set `self.HasAnomaly` false)
    (else
      (bind _output_get (set `self.HasAnomaly` (`KismetMathLibrary.RandomBool`)))
      (if _output_get
        (if (not (> _returnvalue 0))
          (`self.resetArray`))
        (bind _output_get_2 (set `self.randomAnomaly` (`|GetArrayItem` _anomaly_array (`KismetMathLibrary.RandomIntegerInRange` 0 (- _returnvalue 1)))))
        (`KismetSystemLibrary.PrintString` (`KismetStringLibrary.Concat_StrStr` "remove " (`KismetStringLibrary.Conv_IntToString` _output_get_2)))
        (`KismetArrayLibrary.Array_RemoveItem` (`self.Anomaly_array`) _output_get_2)
        (for _array_element (`self.Anomaly_array`)
          (`KismetSystemLibrary.PrintString` (`KismetStringLibrary.Conv_IntToString` _array_element))
          (`KismetSystemLibrary.PrintString` "\"GI VALUE: \" + HasAnomaly"))))))

(fn `resetArray`
  (for _index (range 1 (+ (`self.anomalyNum`) 1))
    (`KismetArrayLibrary.Array_Add` (`self.Anomaly_array`) _index)))