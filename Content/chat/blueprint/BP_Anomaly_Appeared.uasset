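; BP_Anomaly_Appeared is an anomaly actor whose mesh appears only when the game instance flags that an anomaly is active.
; On BeginPlay it applies its configured static mesh, then UpdateAnomaly reads HasAnomaly from BP_MyGameInstance to toggle hidden state and collision.
; BeginPlay then checks the flag again, making the mesh visible or destroying the actor when no anomaly exists.
; Debug prints report startup and the flag's value.
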(event `UpdateAnomaly`
  (bind _asbp_my_game_instance (cast `/Game/chat/blueprint/BP_MyGameInstance` (`GameplayStatics.GetGameInstance`)))
  (`KismetSystemLibrary.PrintString` (`KismetStringLibrary.Conv_BoolToString` (`/Game/chat/blueprint/BP_MyGameInstance.HasAnomaly` _asbp_my_game_instance)))
  (if (`/Game/chat/blueprint/BP_MyGameInstance.HasAnomaly` _asbp_my_game_instance)
    (`SceneComponent.SetHiddenInGame` (`self.MeshDisplay`) false false)
    (`PrimitiveComponent.SetCollisionEnabled` (`self.MeshDisplay`) "QueryAndPhysics")
    (else
      (`SceneComponent.SetHiddenInGame` (`self.MeshDisplay`) true false)
      (`PrimitiveComponent.SetCollisionEnabled` (`self.MeshDisplay`) "NoCollision"))))

(event `self.ReceiveBeginPlay`
  (`StaticMeshComponent.SetStaticMesh` (`self.MeshDisplay`) (`self.MyMesh`))
  (`KismetSystemLibrary.PrintString` "BP_Anomaly BeginPlay")
  (`self.UpdateAnomaly`)
  (bind _asbp_my_game_instance (cast `/Game/chat/blueprint/BP_MyGameInstance` (`GameplayStatics.GetGameInstance`)))
  (if (`/Game/chat/blueprint/BP_MyGameInstance.HasAnomaly` _asbp_my_game_instance)
    (`SceneComponent.SetVisibility` (`self.MeshDisplay`) true false)
    (else
      (`self.K2_DestroyActor`))))

(fn `UserConstructionScript`)