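; Glasses actor for anomaly number 7, which stays in the level only when that anomaly is rolled.
; On BeginPlay it reads HasAnomaly and RandomAnomaly from BP_MyGameInstance, then either hides the mesh without collision or destroys itself.
; Tick polls AnomalyBedGone and, while it is set, shows the glasses with collision restored.
; UpdateAnomaly only prints the HasAnomaly flag, and the construction script does nothing.
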(event `UpdateAnomaly`
  (params (setActive :type Boolean))
  (bind _asbp_my_game_instance (cast `/Game/chat/blueprint/BP_MyGameInstance` (`GameplayStatics.GetGameInstance`)))
  (`KismetSystemLibrary.PrintString` (`KismetStringLibrary.Conv_BoolToString` (`/Game/chat/blueprint/BP_MyGameInstance.HasAnomaly` _asbp_my_game_instance)))
  (if (`/Game/chat/blueprint/BP_MyGameInstance.HasAnomaly` _asbp_my_game_instance)
    _))

(event `glass_appear`
  (bind _meshdisplay (`self.MeshDisplay`))
  (`SceneComponent.SetHiddenInGame` _meshdisplay false false)
  (`PrimitiveComponent.SetCollisionEnabled` _meshdisplay "QueryAndPhysics"))

(event `glass_disappear`
  (bind _meshdisplay (`self.MeshDisplay`))
  (`SceneComponent.SetHiddenInGame` _meshdisplay true false)
  (`PrimitiveComponent.SetCollisionEnabled` _meshdisplay "NoCollision"))

(event `self.ReceiveBeginPlay`
  (`self.UpdateAnomaly` false)
  (bind _asbp_my_game_instance (cast `/Game/chat/blueprint/BP_MyGameInstance` (`GameplayStatics.GetGameInstance`)))
  (if (`/Game/chat/blueprint/BP_MyGameInstance.HasAnomaly` _asbp_my_game_instance)
    (if (== (`/Game/chat/blueprint/BP_MyGameInstance.randomAnomaly` _asbp_my_game_instance) 7)
      (`self.glass_disappear`)
      (else
        (`self.K2_DestroyActor` :!label _label)))
    (else
      (goto _label))))

(event `self.ReceiveTick`
  (params (DeltaSeconds :type "Float (single-precision)"))
  (bind _asbp_my_game_instance (cast `/Game/chat/blueprint/BP_MyGameInstance` (`GameplayStatics.GetGameInstance`)))
  (if (`/Game/chat/blueprint/BP_MyGameInstance.anomalyBedGone` _asbp_my_game_instance)
    (`self.glass_appear`)))

(fn `UserConstructionScript`)