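; BP_Anomaly_door_glass is an anomaly actor that appears only when the game rolls its specific anomaly.
; On BeginPlay it hides its cube, then reads HasAnomaly and RandomAnomaly from BP_MyGameInstance to either show it with collision or destroy itself.
; InteractDoorGlass destroys the actor.
; UpdateAnomaly only prints the anomaly flag and ignores its SetActive input.
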(event `UpdateAnomaly`
  (params (setActive :type Boolean))
  (bind _asbp_my_game_instance (cast `/Game/chat/blueprint/BP_MyGameInstance` (`GameplayStatics.GetGameInstance`)))
  (`KismetSystemLibrary.PrintString` (`KismetStringLibrary.Conv_BoolToString` (`/Game/chat/blueprint/BP_MyGameInstance.HasAnomaly` _asbp_my_game_instance)))
  (if (`/Game/chat/blueprint/BP_MyGameInstance.HasAnomaly` _asbp_my_game_instance)
    _))

(event `InteractDoorGlass`
  (`self.K2_DestroyActor`))

(event `self.ReceiveBeginPlay`
  (bind _cube (`self.Cube`))
  (bind _cube_2 (`self.Cube`))
  (`KismetSystemLibrary.PrintString` "BP_Anomaly BeginPlay")
  (`PrimitiveComponent.SetCollisionEnabled` _cube "NoCollision")
  (`SceneComponent.SetVisibility` _cube false false)
  (`self.UpdateAnomaly` false)
  (bind _asbp_my_game_instance (cast `/Game/chat/blueprint/BP_MyGameInstance` (`GameplayStatics.GetGameInstance`)))
  (if (`/Game/chat/blueprint/BP_MyGameInstance.HasAnomaly` _asbp_my_game_instance)
    (if (== (`/Game/chat/blueprint/BP_MyGameInstance.randomAnomaly` _asbp_my_game_instance) 7)
      (`PrimitiveComponent.SetCollisionEnabled` _cube_2 "QueryAndPhysics")
      (`SceneComponent.SetVisibility` _cube_2 true false)
      (else
        (`self.K2_DestroyActor` :!label _label)))
    (else
      (goto _label))))

(fn `UserConstructionScript`)