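; Anomaly bed actor that exists only when the game instance has anomaly 7 active, destroying itself otherwise.
; On BeginPlay, AnomalyBedAppear sets its cube's visibility and collision, while separate appear and disappear events toggle hidden state and collision.
; InteractBed increments the level if an anomaly is present or resets it to zero, generates the next anomaly, then fades out and opens the stateCheck level.
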(event `InteractBed`
  (bind _asbp_my_game_instance (cast `/Game/chat/blueprint/BP_MyGameInstance` (`GameplayStatics.GetGameInstance`)))
  (set `/Game/chat/blueprint/BP_MyGameInstance.Istransition` true _asbp_my_game_instance)
  (set `/Game/chat/blueprint/BP_MyGameInstance.IsInteract` true _asbp_my_game_instance)
  (if (`/Game/chat/blueprint/BP_MyGameInstance.HasAnomaly` _asbp_my_game_instance)
    (set `/Game/chat/blueprint/BP_MyGameInstance.CurrentLevel` (+ (`/Game/chat/blueprint/BP_MyGameInstance.CurrentLevel` _asbp_my_game_instance) 1) _asbp_my_game_instance)
    (else
      (set `/Game/chat/blueprint/BP_MyGameInstance.CurrentLevel` 0 _asbp_my_game_instance)))
  (`/Game/chat/blueprint/BP_MyGameInstance.GenerateAnomaly` _asbp_my_game_instance)
  (`PlayerCameraManager.StartCameraFade` :`self` (`GameplayStatics.GetPlayerCameraManager` 0) :`ToAlpha` 1.0 :`Duration` 1.5 :`bHoldWhenFinished` true)
  (`KismetSystemLibrary.Delay` 1.5)
  (`GameplayStatics.OpenLevel` "stateCheck")
  (`KismetSystemLibrary.PrintString` "Bed Used"))

(event `disappear`
  (bind _cube (`self.Cube`))
  (`SceneComponent.SetHiddenInGame` _cube true false)
  (`PrimitiveComponent.SetCollisionEnabled` _cube "NoCollision"))

(event `appear`
  (bind _cube (`self.Cube`))
  (`SceneComponent.SetHiddenInGame` _cube false false)
  (`PrimitiveComponent.SetCollisionEnabled` _cube "QueryAndPhysics"))

(event `self.ReceiveBeginPlay`
  (bind _cube (`self.Cube`))
  (bind _cube_2 (`self.Cube`))
  (bind _asbp_my_game_instance (cast `/Game/chat/blueprint/BP_MyGameInstance` (`GameplayStatics.GetGameInstance`)))
  (if (`/Game/chat/blueprint/BP_MyGameInstance.HasAnomaly` _asbp_my_game_instance)
    (if (== (`/Game/chat/blueprint/BP_MyGameInstance.randomAnomaly` _asbp_my_game_instance) 7)
      (bind _asbp_my_game_instance_2 (cast `/Game/chat/blueprint/BP_MyGameInstance` (`GameplayStatics.GetGameInstance`)))
      (if (`/Game/chat/blueprint/BP_MyGameInstance.anomalyBedAppear` _asbp_my_game_instance_2)
        (`PrimitiveComponent.SetCollisionEnabled` _cube_2 "QueryAndPhysics")
        (`SceneComponent.SetVisibility` _cube_2 true false)
        (else
          (`PrimitiveComponent.SetCollisionEnabled` _cube "NoCollision")
          (`SceneComponent.SetVisibility` _cube false false)))
      (else
        (`self.K2_DestroyActor` :!label _label)))
    (else
      (goto _label))))

(fn `UserConstructionScript`)