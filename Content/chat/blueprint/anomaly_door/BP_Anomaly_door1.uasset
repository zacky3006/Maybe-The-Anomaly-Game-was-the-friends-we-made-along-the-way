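; Anomaly door actor that slides away from the player while they are near it, used as one of the game's random anomalies.
; On BeginPlay it stays and shows its mesh only when the game instance has an anomaly with the matching random index; otherwise it destroys itself.
; A box overlap flags player proximity, and Tick pushes the actor horizontally away from the player.
; UpdateAnomaly only prints the anomaly flag.
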(event `UpdateAnomaly`
  (params (setActive :type Boolean))
  (bind _asbp_my_game_instance (cast `/Game/chat/blueprint/BP_MyGameInstance` (`GameplayStatics.GetGameInstance`)))
  (`KismetSystemLibrary.PrintString` (`KismetStringLibrary.Conv_BoolToString` (`/Game/chat/blueprint/BP_MyGameInstance.HasAnomaly` _asbp_my_game_instance)))
  (if (`/Game/chat/blueprint/BP_MyGameInstance.HasAnomaly` _asbp_my_game_instance)
    _))

(event `self.Box.OnComponentBeginOverlap`
  (params (OverlappedComponent :type "PrimitiveComponent Object Reference") (OtherActor :type "Actor Object Reference") (OtherComp :type "PrimitiveComponent Object Reference") (OtherBodyIndex :type Integer) (bFromSweep :type Boolean) (SweepResult :type "HitResult Structure (by ref)"))
  (bind _asbp_first_person_character (cast `/Game/chat/blueprint/BP_FirstPersonCharacter` OtherActor))
  (set `self.bPlayerNear` true))

(event `self.Box.OnComponentEndOverlap`
  (params (OverlappedComponent :type "PrimitiveComponent Object Reference") (OtherActor :type "Actor Object Reference") (OtherComp :type "PrimitiveComponent Object Reference") (OtherBodyIndex :type Integer))
  (cast `/Game/chat/blueprint/BP_FirstPersonCharacter` OtherActor)
  (set `self.bPlayerNear` false))

(event `self.ReceiveTick`
  (params (DeltaSeconds :type "Float (single-precision)"))
  (if (`self.bPlayerNear`)
    (`self.K2_AddActorWorldOffset` (* (* (`KismetMathLibrary.MakeVector` (.x (`KismetMathLibrary.Normal` (- (`self.K2_GetActorLocation`) (`self.K2_GetActorLocation` (`GameplayStatics.GetPlayerCharacter` 0))))) (.y (`KismetMathLibrary.Normal` (- (`self.K2_GetActorLocation`) (`self.K2_GetActorLocation` (`GameplayStatics.GetPlayerCharacter` 0)))))) (`self.float`)) DeltaSeconds))))

(event `self.ReceiveBeginPlay`
  (`self.UpdateAnomaly` false)
  (bind _asbp_my_game_instance (cast `/Game/chat/blueprint/BP_MyGameInstance` (`GameplayStatics.GetGameInstance`)))
  (if (`/Game/chat/blueprint/BP_MyGameInstance.HasAnomaly` _asbp_my_game_instance)
    (if (== (`/Game/chat/blueprint/BP_MyGameInstance.randomAnomaly` _asbp_my_game_instance) 23)
      (`SceneComponent.SetVisibility` (`self.MeshDisplay`) true false)
      (`self.SetActorHiddenInGame` false)
      (else
        (`self.K2_DestroyActor` :!label _label)))
    (else
      (goto _label))))

(fn `UserConstructionScript`)